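; BP_PowerUpShot is a moving pickup that grants the player a timed shot power-up in a space shooter.
; Each Tick, MovePU moves it along the forward vector captured at BeginPlay, and it destroys itself after a fixed delay.
; Overlapping a Player-tagged actor destroys it and sets that character's PowerUpEndTime a few seconds ahead of game time.
; An older PowerUpShotActive toggle with timer and delay variants remains as mostly unconnected nodes.
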(event Custom|DisablePowerUpShot
  (Variables|/Game/Players/BP_SpaceS_Character.BP_SpaceS_Character_C|SetbPowerUpShotActive (stale Collision|EventActorBeginOverlap _asbp_space_s_character) false)
  (Development|PrintString "POWER UP FALSE"))

(event EventBeginPlay
  (Variables|Default|SetMovement (Transformation|GetActorForwardVector))
  (Utilities|FlowControl|Delay 7.0)
  (Actor|DestroyActor)
  (Variables|/Game/Players/BP_SpaceS_Character.BP_SpaceS_Character_C|SetPowerUpEndTime (stale Collision|EventActorBeginOverlap _asbp_space_s_character) 0.0))

(event Collision|EventActorBeginOverlap
  (params (OtherActor :type Actor%20Object%20Reference))
  (if (Actor|ActorHasTag OtherActor "Player")
    (Actor|DestroyActor)
    (bind _asbp_space_s_character (Utilities|Casting|CastToBP_SpaceS_Character OtherActor))
    (Variables|/Game/Players/BP_SpaceS_Character.BP_SpaceS_Character_C|SetPowerUpEndTime _asbp_space_s_character (+ (Utilities|Time|GetGameTimeinSeconds) 5.0))))

(event EventTick
  (params (DeltaSeconds :type Float%20%28single-precision%29))
  (CallFunction|MovePU DeltaSeconds))

(fn ConstructionScript)

(fn MovePU
  (params (DeltaTime :type Float%20%28double-precision%29))
  (Transformation|SetActorLocation (+ (Transformation|GetActorLocation) (* (* DeltaTime (Variables|Default|GetSpeedPUL)) (Variables|Default|GetMovement))) false false))