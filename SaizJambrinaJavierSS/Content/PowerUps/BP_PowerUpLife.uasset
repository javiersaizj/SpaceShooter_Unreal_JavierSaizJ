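; Extra-life power-up that travels in a straight line and is collected by overlapping the player.
; BeginPlay stores the actor's forward vector as its direction and destroys it after a fixed delay, while Tick moves it along that vector by speed and delta time, without sweep.
; An overlap with a Player-tagged BP_SpaceS_Character adds a life if the count is within the limit, and destroys the pickup either way.
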(event EventBeginPlay
  (Variables|Default|SetMovement (Transformation|GetActorForwardVector))
  (Utilities|FlowControl|Delay 7.0)
  (Actor|DestroyActor))

(event Collision|EventActorBeginOverlap
  (params (OtherActor :type Actor%20Object%20Reference))
  (if (Actor|ActorHasTag OtherActor "Player")
    (bind _asbp_space_s_character (Utilities|Casting|CastToBP_SpaceS_Character OtherActor))
    (if (<= (Variables|/Game/Players/BP_SpaceS_Character.BP_SpaceS_Character_C|GetLifes _asbp_space_s_character) 3)
      (Variables|/Game/Players/BP_SpaceS_Character.BP_SpaceS_Character_C|SetLifes _asbp_space_s_character (+ (Variables|/Game/Players/BP_SpaceS_Character.BP_SpaceS_Character_C|GetLifes _asbp_space_s_character) 1))
      (Actor|DestroyActor)
      (else
        (Actor|DestroyActor)))))

(event EventTick
  (params (DeltaSeconds :type Float%20%28single-precision%29))
  (CallFunction|MovePU DeltaSeconds))

(fn ConstructionScript)

(fn MovePU
  (params (DeltaTime :type Float%20%28double-precision%29))
  (Transformation|SetActorLocation (+ (Transformation|GetActorLocation) (* (* DeltaTime (Variables|Default|GetSpeedPUL)) (Variables|Default|GetMovement))) false false))