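; BP_SS_GameMode is a game mode that tracks run progress, enemy kills and the level.
; Tick adds a fixed increment to Progress every frame.
; Each EnemyDestroyed event raises the kill count, and every second kill raises Level.
; PlayerDead casts the first player's HUD to BP_SSHUD and calls its player-dead UI.
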(event Custom|PlayerDead
  (bind _asbp_sshud (Utilities|Casting|CastToBP_SSHUD (HUD|GetHUD (Game|GetPlayerController 0))))
  (Default|PlayerDeadUI _asbp_sshud))

(event Custom|EnemyDestroyed
  (bind _output_get (Variables|Default|SetEnemiesDestroyed (+ (Variables|Default|GetEnemiesDestroyed) 1)))
  (if (== (Math|Integer|%(Integer) _output_get 2) 0)
    (Variables|Default|SetLevel (+ (Variables|Default|GetLevel) 1))))

(event EventBeginPlay)

(event EventTick
  (params (DeltaSeconds :type Float%20%28single-precision%29))
  (Variables|Default|SetProgress (+ (Variables|Default|GetProgress) (Variables|Default|GetIncrementPerTick))))

(fn ConstructionScript)