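; Player ship character for a space shooter, using Enhanced Input to move within a clamped flat play area, with flipbooks for left, right and idle.
; Timer-gated firing spawns Ammo from two spawn points, or four until PowerUpEndTime passes.
; Enemy overlaps remove a life after a short delay that ignores further hits.
; At zero lives it pauses, notifies BP_SS_GameMode and switches to UI input.
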(event Custom|UpdateFire
  (Variables|Default|SetCanFire true))

(event Custom|DamageActor
  (bind _output_get (Variables|Default|SetLifes (- (Variables|Default|GetLifes) 1)))
  (if (== _output_get 0)
    (Game|SetGamePaused true)
    (bind _asbp_ss_game_mode (Utilities|Casting|CastToBP_SS_GameMode (Game|GetGameMode)))
    (Default|PlayerDead _asbp_ss_game_mode)
    (Variables|/Script/Engine.PlayerController|SetbShowMouseCursor (Game|GetPlayerController 0) true)
    (Input|SetInputModeUIOnly (Game|GetPlayerController 0) 0 "DoNotLock" false)))

(event Input|EnhancedActionEvents|EnhancedInputActionBP_InputFire
  (params (ActionValue :type Boolean) (ElapsedSeconds :type Float%20%28double-precision%29) (TriggeredSeconds :type Float%20%28double-precision%29) (InputAction :type Input%20Action%20Object%20Reference :default "/Game/Inputs/BP_InputFire.BP_InputFire"))
  (:Triggered
    (if (Variables|Default|GetCanFire)
      (CallFunction|DoFire)
      (Variables|Default|SetCanFire false)
      (Utilities|Time|SetTimerbyEvent (delegate Custom|UpdateFire) (Variables|Default|GetFireDelay)))))

(event Input|EnhancedActionEvents|EnhancedInputActionBP_InputMove
  (params (ActionValue :type Vector%202D%20Structure) (ElapsedSeconds :type Float%20%28double-precision%29) (TriggeredSeconds :type Float%20%28double-precision%29) (InputAction :type Input%20Action%20Object%20Reference :default "/Game/Inputs/BP_InputMove.BP_InputMove"))
  (bind _returnvalue (Transformation|GetActorLocation))
  (bind (_x _y) (Math|Vector|BreakVector _returnvalue))
  (:Triggered
    (Pawn|Input|AddMovementInput (Transformation|GetActorRightVector) (.x ActionValue) false)
    (Pawn|Input|AddMovementInput (Math|Vector|GetForwardVector "0, 0, 0") (.y ActionValue) false)
    (Transformation|SetActorLocation (Math|Vector|MakeVector (Math|Float|Clamp(Float) _x -3.5e+02 3.5e+02) (Math|Float|Clamp(Float) _y -6.5e+02 6.5e+02) 0.0) false false)))

(event EventBeginPlay
  (bind _asplayer_controller (Utilities|Casting|CastToPlayerController (Pawn|GetController)))
  (Utilities|IsValid (PlayerController|LocalPlayerSubsystems|GetEnhancedInputLocalPlayerSubsystem _asplayer_controller)
    (:Is%20Valid
      (Input|AddMappingContext (PlayerController|LocalPlayerSubsystems|GetEnhancedInputLocalPlayerSubsystem _asplayer_controller) "/Game/Inputs/BP_InputMapping.BP_InputMapping" 0 "(bIgnoreAllPressedKeysUntilRelease=True,bForceImmediately=False)"))))

(event Collision|EventActorBeginOverlap
  (params (OtherActor :type Actor%20Object%20Reference))
  (Utilities|IsValid OtherActor
    (:Is%20Valid
      (if (Actor|ActorHasTag OtherActor "Enemy")
        (if (Variables|Default|GetCanTakeDamage)
          (Variables|Default|SetCanTakeDamage false)
          (Utilities|FlowControl|Delay 0.3)
          (Variables|Default|SetCanTakeDamage true)
          (if (Variables|Default|GetCanTakeDamage)
            (CallFunction|DamageActor)))))))

(event EventTick
  (params (DeltaSeconds :type Float%20%28single-precision%29)))

(event Input|ActionEvents|InputActionMoverIzq
  (params (Key :type Key%20Structure :default "None"))
  (bind _sprite (Variables|Default|GetSprite))
  (:Pressed
    (Variables|Default|SetMovingLeft true)
    (Sprite|SetFlipbook _sprite "/Game/Images/Player/PLAYER_IZQ.PLAYER_IZQ"))
  (:Released
    (Variables|Default|SetMovingLeft false)
    (if (not (Variables|Default|GetMovingRight))
      (Sprite|SetFlipbook _sprite "/Game/Images/Player/PLAYER_IDLE.PLAYER_IDLE"))))

(event Input|ActionEvents|InputActionMoverDerecha
  (params (Key :type Key%20Structure :default "None"))
  (bind _sprite (Variables|Default|GetSprite))
  (:Pressed
    (Variables|Default|SetMovingRight true)
    (Sprite|SetFlipbook _sprite "/Game/Images/Player/PLAYER_DERECHA.PLAYER_DERECHA"))
  (:Released
    (Variables|Default|SetMovingRight false)
    (if (not (Variables|Default|GetMovingLeft))
      (Sprite|SetFlipbook _sprite "/Game/Images/Player/PLAYER_IDLE.PLAYER_IDLE"))))

(fn ConstructionScript)

(fn DoFire
  (if (<= (Utilities|Time|GetGameTimeinSeconds) (Variables|Default|GetPowerUpEndTime))
    (Game|SpawnActorfromClass (Variables|Default|GetAmmo) (Transformation|GetWorldTransform (Variables|Default|GetSpawnDisparo)) "Undefined" 0 0)
    (Game|SpawnActorfromClass (Variables|Default|GetAmmo) (Transformation|GetWorldTransform (Variables|Default|GetSpawnDisparo2)) "Undefined" 0 0)
    (Game|SpawnActorfromClass (Variables|Default|GetAmmo) (Transformation|GetWorldTransform (Variables|Default|GetSpawnDisparo3)) "Undefined" 0 0)
    (Game|SpawnActorfromClass (Variables|Default|GetAmmo) (Transformation|GetWorldTransform (Variables|Default|GetSpawnDisparo4)) "Undefined" 0 0)
    (else
      (Game|SpawnActorfromClass (Variables|Default|GetAmmo) (Transformation|GetWorldTransform (Variables|Default|GetSpawnDisparo)) "Undefined" 0 0)
      (Game|SpawnActorfromClass (Variables|Default|GetAmmo) (Transformation|GetWorldTransform (Variables|Default|GetSpawnDisparo2)) "Undefined" 0 0))))